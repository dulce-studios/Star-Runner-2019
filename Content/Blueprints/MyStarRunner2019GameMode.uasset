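; Game mode for a StarRunner game, holding logic to spawn the initial hallway at the player start.
; SpawnInitialHallway spawns a Hallway_x3 slightly below the player start, matching its rotation with a large uniform scale, and returns it.
; The graph nodes that call it and then trigger SpawnLeft and SpawnRight on the hallway are unconnected, so BeginPlay and Tick do nothing.
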(event EventBeginPlay)

(event EventTick
  (params (DeltaSeconds :type Float%20%28single-precision%29)))

(fn ConstructionScript)

(fn SpawnInitialHallway
  (bind _returnvalue (Class|GameModeBase|FindPlayerStart))
  (bind _rootcomponent (Variables|/Script/Engine.Actor|GetRootComponent _returnvalue))
  (bind _returnvalue_2 (Transformation|GetWorldTransform _rootcomponent))
  (bind (_location _rotation) (Math|Transform|BreakTransform _returnvalue_2))
  (bind _returnvalue_3 (Game|SpawnActorfromClass "/Game/Blueprints/hallway_x3.hallway_x3_C" (Math|Transform|MakeTransform (+ _location "0, 0,-120.000000") _rotation "50.000000,50.000000,50.000000") "Undefined" 0 0))
  (return _returnvalue_3))