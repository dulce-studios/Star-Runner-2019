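; Hallway_x3 is a self-spawning hallway segment that builds a branching left/right corridor around the first-person player.
; Entering its trigger enables the player's left/right tracking and has both child hallways spawn their own children at offsets from their arrow components.
; Leaving it destroys the branch not taken (judged by WentLeft) along with its children, then the segment itself, keeping only a small window of the binary tree loaded.
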(event OnComponentEndOverlap(SpawnTrigger)
  (params (OverlappedComponent :type Primitive%20Component%20Object%20Reference) (OtherActor :type Actor%20Object%20Reference) (OtherComp :type Primitive%20Component%20Object%20Reference) (OtherBodyIndex :type Integer))
  (if (Utilities|ClassIsChildOf (Utilities|GetClass OtherActor) "/Game/Blueprints/FirstPersonCharacter.FirstPersonCharacter_C")
    (bind _asfirst_person_character (Utilities|Casting|CastToFirstPersonCharacter OtherActor)
      (:then
        (if (Variables|/Game/Blueprints/FirstPersonCharacter.FirstPersonCharacter_C|GetwentLeft _asfirst_person_character)
          (CallFunction|DestroywithFACTSandLOGIC (Variables|Default|GetRightChildHallway))
          (else
            (CallFunction|DestroywithFACTSandLOGIC (Variables|Default|GetLeftChildHallway))))
        (Actor|DestroyActor))
      (:CastFailed
        (Class|VisualLoggerKismetLibrary|LogText 0 "" "VisLogBP")))))

(event OnComponentBeginOverlap(SpawnTrigger)
  (params (OverlappedComponent :type Primitive%20Component%20Object%20Reference) (OtherActor :type Actor%20Object%20Reference) (OtherComp :type Primitive%20Component%20Object%20Reference) (OtherBodyIndex :type Integer) (bFromSweep :type Boolean) (SweepResult :type Hit%20Result%20Structure%20%28by%20ref%29))
  (if (Utilities|ClassIsChildOf (Utilities|GetClass OtherActor) "/Game/Blueprints/FirstPersonCharacter.FirstPersonCharacter_C")
    (bind _asfirst_person_character (Utilities|Casting|CastToFirstPersonCharacter OtherActor))
    (Variables|/Game/Blueprints/FirstPersonCharacter.FirstPersonCharacter_C|SetenableLeftRight _asfirst_person_character true)
    (CallFunction|SpawnGrandchildren (Variables|Default|GetLeftChildHallway))
    (CallFunction|SpawnGrandchildren (Variables|Default|GetRightChildHallway))))

(fn ConstructionScript)

(fn SpawnRight
  (bind _rightarrow (Variables|Default|GetRightArrow))
  (bind _returnvalue (Transformation|GetWorldTransform _rightarrow))
  (bind (_location _rotation) (Math|Transform|BreakTransform _returnvalue))
  ;[1 1 1] SAD
  (bind _returnvalue_2 (Game|SpawnActorfromClass "hallway_x3_C" (Math|Transform|MakeTransform (+ _location (Math|Vector|RotateVector (Math|Vector|MakeVector 2.5e+02 0.0 0.0) _rotation)) _rotation (Transformation|GetActorScale3D)) "AlwaysSpawn" 0 0))
  (Variables|Default|SetRightChildHallway _returnvalue_2))

(fn SpawnLeft
  (bind _leftarrow (Variables|Default|GetLeftArrow))
  (bind _returnvalue (Transformation|GetWorldTransform _leftarrow))
  (bind (_location _rotation) (Math|Transform|BreakTransform _returnvalue))
  ;[1 1 1] SAD
  (bind _returnvalue_2 (Game|SpawnActorfromClass "hallway_x3_C" (Math|Transform|MakeTransform (+ _location (Math|Vector|RotateVector (Math|Vector|MakeVector 2.5e+02 0.0 0.0) _rotation)) _rotation (Transformation|GetActorScale3D)) "AlwaysSpawn" 0 0))
  (Variables|Default|SetLeftChildHallway _returnvalue_2))

(fn SpawnGrandchildren
  (params (Hallway :type Hallway%20X%203%20Object%20Reference%20%28by%20ref%29))
  (CallFunction|SpawnLeft Hallway)
  (CallFunction|SpawnRight Hallway))

(fn DestroywithFACTSandLOGIC
  (Utilities|FlowControl|Sequence
    (:then_0
      (Actor|DestroyActor (Variables|Default|GetLeftChildHallway)))
    (:then_1
      (Actor|DestroyActor (Variables|Default|GetRightChildHallway)))
    (:then_2
      (Actor|DestroyActor))))